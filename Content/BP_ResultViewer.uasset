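; BP_ResultViewer is an actor that fetches the new-books listing from the itbook.store web API and shows the response in its widget component.
; On BeginPlay it creates a WBP_ResultViewer widget and assigns it to that component.
; An actor overlap sends the GET request through SendRequest with a hard-coded URL and path.
; The RequestWriteBack event writes the returned result into the widget's MText as plain text.
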(event EventBeginPlay
  (bind _returnvalue (UserInterface|CreateWidget "/RESTReceiver/WBP_ResultViewer.WBP_ResultViewer_C"))
  (UserInterface|SetWidget (Variables|Default|GetWidget) _returnvalue))

(event Collision|EventActorBeginOverlap
  (params (OtherActor :type Actor%20Object%20Reference))
  (Class|HttpReceiver|SendRequest (Utilities|String|MakeLiteralString "https://api.itbook.store") (Utilities|String|MakeLiteralString "GET") (Utilities|String|MakeLiteralString "/1.0/new")))

(event EventTick
  (params (DeltaSeconds :type Float%20%28single-precision%29)))

(event EventRequestWriteBack
  (params (Result :type String%20%28by%20ref%29))
  (Variables|/Script/UMG.TextBlock|SetText (Variables|/Script/RESTReceiver.HttpViewer|Getm_text (.AsWBP%20Result%20Viewer (Utilities|Casting|CastToWBP_ResultViewer (UserInterface|GetUserWidgetObject (Variables|Default|GetWidget))))) (Utilities|Text|ToText(String) Result)))

(fn ConstructionScript)